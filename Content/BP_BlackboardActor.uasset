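; Blackboard actor that displays a hard-coded Japanese multiple-choice reading question as 3D text, built entirely in the construction script.
; The template Text3D is sized to the Box bounds and moved to its upper-left corner, nudged off the board surface.
; The question string is parsed into pieces, each spawning a Text3D component stacked downward at box-relative spacing and copying the template's font, scale, width and extrusion.
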(event EventBeginPlay)

(event Collision|EventActorBeginOverlap
  (params (OtherActor :type Actor%20Object%20Reference)))

(fn ConstructionScript
  (bind _box (Variables|Default|GetBox))
  (bind _text3d (Variables|Default|GetText3D))
  (bind _boxextent (Collision|GetComponentBounds _box))
  (bind _returnvalue (Transformation|GetWorldLocation _box))
  (bind _returnvalue_2 (Transformation|GetWorldLocation _text3d))
  ;[1 1 1] Move text to the upper left corner
  (Class|Text3DComponent|SetMaxWidth (Variables|Default|GetText3D) (* (/ 1.0 (.x (Variables|/Script/Engine.SceneComponent|GetRelativeScale3D (Variables|Default|GetText3D)))) 2.0 (.x _boxextent)))
  (Transformation|SetWorldLocation (Variables|Default|GetText3D) (Math|Vector|MakeVector (- (.x _returnvalue) (.x _boxextent)) (+ (.y _returnvalue) 2.001) (+ (.z _returnvalue) (.z _boxextent))) false false)
  (for (_array_element _array_index) (Utilities|String|ParseIntoArray "新しい　くるまですね。 
 
１　あたらしい 
２　あだらしい 
３　あらたしい 
４　あらだしい" " 
")
    (bind _returnvalue_3 (AddComponent|AddText3DComponent self false))
    (bind _output_get (LocalVariables|SetInstantiated%20Text3D _returnvalue_3))
    (Class|Text3DComponent|SetFont _output_get (Variables|/Script/Text3D.Text3DComponent|GetFont (Variables|Default|GetText3D)))
    (Class|Text3DComponent|SetText (LocalVariables|GetInstantiated%20Text3D) (Utilities|Text|ToText(String) (Utilities|String|MakeLiteralString _array_element)))
    (Transformation|SetWorldLocation (LocalVariables|GetInstantiated%20Text3D) (Math|Vector|MakeVector (.x _returnvalue_2) (.y _returnvalue_2) (- (.z _returnvalue_2) (* (+ _array_index 1) (/ (.z (.BoxExtent (Collision|GetComponentBounds (Variables|Default|GetBox)))) 3.0)))) false false)
    (Class|Text3DComponent|SetHasMaxHeight (LocalVariables|GetInstantiated%20Text3D) false)
    (Class|Text3DComponent|SetHasMaxWidth (LocalVariables|GetInstantiated%20Text3D) true)
    (Class|Text3DComponent|SetMaxWidth (LocalVariables|GetInstantiated%20Text3D) (Variables|/Script/Text3D.Text3DComponent|GetMaxWidth (Variables|Default|GetText3D)))
    (Class|Text3DComponent|SetVerticalAlignment (LocalVariables|GetInstantiated%20Text3D) "Top")
    (Transformation|SetRelativeScale3D (LocalVariables|GetInstantiated%20Text3D) (Variables|/Script/Engine.SceneComponent|GetRelativeScale3D (Variables|Default|GetText3D)))
    (Class|Text3DComponent|SetExtrude (LocalVariables|GetInstantiated%20Text3D) (Variables|/Script/Text3D.Text3DComponent|GetExtrude (Variables|Default|GetText3D)))))